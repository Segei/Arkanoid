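; BP_GameRule is the Arkanoid game rule actor that shows the end-of-game screens.
; On BeginPlay it binds handlers to the OnLoss and OnWin events, skipping this on dedicated servers.
; Each handler creates the matching loss or win widget with itself passed as GameRules, adds it to the viewport and shows the mouse cursor for player controller 0.
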(event Custom|OnLosses
  (bind _returnvalue (UserInterface|CreateWidget "/Game/Arkanoid/HUD/BP_LossWindow.BP_LossWindow_C" 0 self))
  (UserInterface|Viewport|AddtoViewport _returnvalue 0)
  (Variables|/Script/Engine.PlayerController|SetbShowMouseCursor (Game|GetPlayerController 0) true))

(event Custom|OnWining
  (bind _returnvalue (UserInterface|CreateWidget "/Game/Arkanoid/HUD/BP_WinWindow.BP_WinWindow_C" 0 self))
  (UserInterface|Viewport|AddtoViewport _returnvalue 0)
  (Variables|/Script/Engine.PlayerController|SetbShowMouseCursor (Game|GetPlayerController 0) true))

(event EventBeginPlay
  (if (not (Networking|IsDedicatedServer))
    (EventDispatchers|BindEventtoOnLoss (delegate Custom|OnLosses))
    (EventDispatchers|BindEventtoOnWin (delegate Custom|OnWining))))

(fn ConstructionScript)