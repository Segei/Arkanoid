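; Arkanoid cube that spawns a bonus actor when destroyed.
; On BeginPlay it binds to the cube-destroy event, which continues only if the hitting actor is a ball.
; The handler spawns the configured Bonus class at the cube's transform.
; For a BP_Bonuses instance, it sets Direction from the normalized X location of the ball's owner, tying bonus travel to that owner's position.
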(event Custom|CustomEvent_0
  (params (Sendler :type Actor%20Object%20Reference) (HitActor :type Actor%20Object%20Reference))
  (bind _self self)
  (bind _returnvalue (Transformation|GetActorTransform _self))
  (bind _asball_actor (Utilities|Casting|CastToBallActor HitActor))
  (bind _returnvalue_2 (Game|SpawnActorfromClass (Variables|Default|GetBonus) (Math|Transform|MakeTransform (.location _returnvalue) (.rotation _returnvalue) "1.000000,1.000000,1.000000") "Undefined" 0 0))
  (bind _asbp_bonuses (Utilities|Casting|CastToBP_Bonuses _returnvalue_2))
  (Variables|/Game/Arkanoid/Actors/BP_Bonuses.BP_Bonuses_C|SetDirection _asbp_bonuses (Math|Vector|Normalize (Math|Vector|MakeVector (.x (.location (Transformation|GetActorTransform (Components|GetOwner _asball_actor)))) 0.0 0.0))))

(event EventBeginPlay
  (|CallParentFunction)
  (EventDispatchers|BindEventtoOnCubeDestroy (delegate Custom|CustomEvent_0)))

(event Collision|EventActorBeginOverlap
  (params (OtherActor :type Actor%20Object%20Reference))
  (|CallParentFunction OtherActor) ; This node is disabled and will not be called.\nDrag off pins to build functionality.
)

(event EventTick
  (params (DeltaSeconds :type Float%20%28single-precision%29))
  (|CallParentFunction DeltaSeconds) ; This node is disabled and will not be called.\nDrag off pins to build functionality.
)

(fn ConstructionScript
  (|CallParentFunction))