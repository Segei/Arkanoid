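; BP_Bonuses is a moving Arkanoid bonus pickup that applies itself to the RocketPlatform it hits.
; Each Tick sweeps its Sphere along Direction at Speed, with no delta-time scaling, and checks the hit through a collapsed graph.
; A RocketPlatform hit calls AddBonusPlatform, then destroys the actor.
; AddBonusPlatform is empty here, so this Blueprint itself grants no effect.
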(event Custom|AddBonusPlatform
  (params (Platform :type Rocket%20Platform%20Object%20Reference)))

(event EventTick
  (params (DeltaSeconds :type Float%20%28single-precision%29))
  (bind _sweephitresult (Transformation|AddWorldOffset (Variables|Default|GetSphere) (* (Variables|Default|GetDirection) (Variables|Default|GetSpeed)) true false))
  (Utilities|IsValid (|CollapseGraph _sweephitresult)
    (:Is%20Valid
      (bind _asrocket_platform (Utilities|Casting|CastToRocketPlatform (|CollapseGraph _sweephitresult)))
      (CallFunction|AddBonusPlatform _asrocket_platform)
      (Actor|DestroyActor))))

(fn ConstructionScript)