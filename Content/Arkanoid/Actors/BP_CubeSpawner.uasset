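; BP_CubeSpawner is an Arkanoid actor that lays out a grid of cube meshes in its construction script.
; Nested X/Y loops add a static mesh component per cell, offset by cube size plus padding and scaled to that size, then store it in NewVar.
; BeginPlay destroys every stored component, and no replacement cubes are spawned in this graph.
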(event EventBeginPlay
  (for _array_element (Variables|Default|GetNewVar)
    (Components|DestroyComponent _array_element)))

(event Collision|EventActorBeginOverlap
  (params (OtherActor :type Actor%20Object%20Reference)))

(event EventTick
  (params (DeltaSeconds :type Float%20%28single-precision%29)))

(fn ConstructionScript
  (bind _padding (Variables|Default|GetPadding))
  (bind _sizecube (Variables|Default|GetSizeCube))
  (for _index (range (Variables|Default|GetStartX) (Variables|Default|GetX))
    (for _index_2 (range (Variables|Default|GetStartY) (Variables|Default|GetY))
      (bind _returnvalue (AddComponent|AddStaticMeshComponent false (Math|Transform|MakeTransform (Math|Vector|MakeVector (+ (* _index (.x _sizecube)) (* (.x _padding) _index)) (+ (* _index_2 (.y _sizecube)) (* (.y _padding) _index_2)) 0.0) "0, 0, 0" (Math|Vector|MakeVector (/ (.x _sizecube) 1e+02) (/ (.y _sizecube) 1e+02) 1.0))))
      (Utilities|Array|Add (Variables|Default|GetNewVar) _returnvalue))))