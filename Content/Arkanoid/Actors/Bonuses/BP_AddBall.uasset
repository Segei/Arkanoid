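; BP_AddBall is an Arkanoid bonus actor that grants the platform an extra ball to spawn.
; Its AddBonusPlatform event receives the platform and increments that platform's CountSpawnBall counter by one.
; The default BeginPlay, overlap and Tick events are disabled, and the construction script only calls its parent.
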(event EventBeginPlay
  (|CallParentFunction) ; This node is disabled and will not be called.\nDrag off pins to build functionality.
)

(event Collision|EventActorBeginOverlap
  (params (OtherActor :type Actor%20Object%20Reference))
  (|CallParentFunction OtherActor) ; This node is disabled and will not be called.\nDrag off pins to build functionality.
)

(event EventTick
  (params (DeltaSeconds :type Float%20%28single-precision%29))
  (|CallParentFunction DeltaSeconds) ; This node is disabled and will not be called.\nDrag off pins to build functionality.
)

(event EventAddBonusPlatform
  (params (Platform :type Rocket%20Platform%20Object%20Reference))
  (bind _result (Math|Integer|IncrementInt (Variables|/Script/Arkanoid.RocketPlatform|GetCountSpawnBall Platform))
    (:%20%20
      (Variables|/Script/Arkanoid.RocketPlatform|SetCountSpawnBall Platform _result))))

(fn ConstructionScript
  (|CallParentFunction))