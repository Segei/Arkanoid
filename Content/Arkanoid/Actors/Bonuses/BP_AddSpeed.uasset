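; BP_AddSpeed is an Arkanoid bonus actor that changes the speed of the player's platform.
; It handles the AddBonusPlatform event by multiplying the received platform's Speed by its Mult variable.
; The change has no timer or revert here, and the other events are disabled stubs.
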(event EventBeginPlay
  (|CallParentFunction) ; This node is disabled and will not be called.\nDrag off pins to build functionality.
)

(event Collision|EventActorBeginOverlap
  (params (OtherActor :type Actor%20Object%20Reference))
  (|CallParentFunction OtherActor) ; This node is disabled and will not be called.\nDrag off pins to build functionality.
)

(event EventTick
  (params (DeltaSeconds :type Float%20%28single-precision%29))
  (|CallParentFunction DeltaSeconds) ; This node is disabled and will not be called.\nDrag off pins to build functionality.
)

(event EventAddBonusPlatform
  (params (Platform :type Rocket%20Platform%20Object%20Reference))
  (Variables|/Script/Arkanoid.RocketPlatform|SetSpeed Platform (* (Variables|/Script/Arkanoid.RocketPlatform|GetSpeed Platform) (Variables|Default|GetMult))))

(fn ConstructionScript
  (|CallParentFunction))